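; Spell projectile actor configured by a spell data asset that damages what it hits.
; Construction applies the asset's mesh, element materials, speed and homing to the movement and Niagara components, with Flare spells showing a trail effect instead of the mesh.
; Homing spells briefly fly straight before seeking their target component.
; Impact or lifetime timeout detonates it with burst effect and sound, and the actor is destroyed when the burst finishes.
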(event OnSystemFinished(NS_SpellBurst)
  (params (PSystem :type Niagara%20Component%20Object%20Reference))
  (Actor|DestroyActor self))

(event EventBeginPlay
  (bind _projectilemovement (Variables|Default|GetProjectileMovement))
  (CallFunction|PlayCastSFX)
  (bind _spelldataasset (Variables|Default|GetSpellDataAsset)
    (:then
      (if (Variables|/Script/Sigil.DA_SpellInfo|GetbIsHoming _spelldataasset)
        (Variables|/Script/Engine.ProjectileMovementComponent|SetbIsHomingProjectile _projectilemovement false)
        (Utilities|FlowControl|Delay 0.3)
        (Variables|/Script/Engine.ProjectileMovementComponent|SetbIsHomingProjectile _projectilemovement true)))
    (:else)))

(event EventTick
  (params (DeltaSeconds :type Float%20%28single-precision%29))
  (bind _output_get (Variables|Default|SetProjectileLifetime (+ DeltaSeconds (Variables|Default|GetProjectileLifetime))))
  (if (>= _output_get (Variables|Default|GetProjectileTimeout))
    (Utilities|FlowControl|DoOnce false
      (:Completed
        (CallFunction|DetonateProjectile)))))

(event Collision|EventHit
  (params (MyComp :type Primitive%20Component%20Object%20Reference) (Other :type Actor%20Object%20Reference) (OtherComp :type Primitive%20Component%20Object%20Reference) (bSelfMoved :type Boolean) (HitLocation :type Vector :default "0, 0, 0") (HitNormal :type Vector :default "0, 0, 0") (NormalImpulse :type Vector :default "0, 0, 0") (Hit :type Hit%20Result%20Structure%20%28by%20ref%29))
  (Game|Damage|ApplyDamage Other (.DamageAmount (Utilities|Struct|BreakSpellElements (Utilities|Array|Get(acopy) (Variables|/Script/Sigil.DA_SpellInfo|GetSpellDamage (Variables|Default|GetSpellDataAsset))))) (Game|GetInstigatorController) (Game|GetInstigator) "/Script/Engine.DamageType")
  (CallFunction|DetonateProjectile))

(fn ConstructionScript
  (MagicProperties||SetMagicProperties))

(fn SetMagicProperties
  (bind _spelldataasset (Variables|Default|GetSpellDataAsset)
    (:then
      (MagicProperties|MagicElementMaterials||ApplySpellMaterials (Variables|/Script/Sigil.DA_SpellInfo|GetMagicElementMaterials _spelldataasset))
      (MagicProperties|StaticMesh|ApplyMeshes (Variables|/Script/Sigil.DA_SpellInfo|GetMesh _spelldataasset))
      (MagicProperties|Movement|SetProjectileSpeeds)
      (MagicProperties|Movement|ConfigureProjectileHoming (Variables|/Script/Sigil.DA_SpellInfo|GetbIsHoming _spelldataasset))
      (if (Utilities|Enum|Equal(Enum) "Flare" (Variables|/Script/Sigil.DA_SpellInfo|GetForm _spelldataasset))
        (Components|Activation|SetAutoActivate (Variables|Default|GetNS_Flare) true)
        (Development|SetHiddeninGame (Variables|Default|GetSpellMesh) true false)))
    (:else)))

(fn PlayCastSFX
  (Audio|SpawnSoundatLocation (Variables|/Script/Sigil.DA_SpellInfo|GetCastSFX (Variables|Default|GetSpellDataAsset)) (Transformation|GetWorldLocation (Variables|Default|GetSpellMesh)) "0, 0, 0" 1.0 1.0 0.0 0 0))

(fn PlayHitSFX
  (Audio|SpawnSoundatLocation (Variables|/Script/Sigil.DA_SpellInfo|GetHitSFX (Variables|Default|GetSpellDataAsset)) (Transformation|GetWorldLocation (Variables|Default|GetSpellMesh)) "0, 0, 0" 1.0 1.0 0.0 0 0))

(fn DetonateProjectile
  (bind _spellmesh (Variables|Default|GetSpellMesh))
  (Components|Activation|Activate (Variables|Default|GetNS_SpellBurst) false)
  (Rendering|SetVisibility _spellmesh false false)
  (Collision|SetCollisionEnabled _spellmesh "NoCollision")
  (CallFunction|PlayHitSFX)
  (Components|Activation|Deactivate (Variables|Default|GetNS_Flare)))

(fn ApplySpellMaterials
  (params (MagicElementMaterials :type Magic%20Element%20Materials%20Structure))
  (MagicProperties|MagicElementMaterials|Mesh|ApplyMeshMaterials MagicElementMaterials)
  (MagicProperties|MagicElementMaterials|FX|ApplyFXMaterialsSpellBurst MagicElementMaterials)
  (MagicProperties|MagicElementMaterials|FX|ApplyFXMaterialsFlare MagicElementMaterials))

(fn ApplyMeshMaterials
  (params (MagicElementMaterials :type Magic%20Element%20Materials%20Structure))
  (Rendering|Material|SetMaterial (Variables|Default|GetSpellMesh) 0 (.MagicElementMaterial (Utilities|Struct|BreakMagicElementMaterials MagicElementMaterials))))

(fn ApplyFXMaterialsSpellBurst
  (params (MagicElementMaterials :type Magic%20Element%20Materials%20Structure))
  (Class|NiagaraComponent|SetVariableMaterial (Variables|Default|GetNS_SpellBurst) "BurstMaterial" (.MagicElementMaterialEmissive (Utilities|Struct|BreakMagicElementMaterials MagicElementMaterials))))

(fn ApplyFXMaterialsFlare
  (params (MagicElementMaterials :type Magic%20Element%20Materials%20Structure))
  (bind (_magicelementmaterial _magicelementmaterialemissive _magicprimarycolour _magicsecondarycolour) (Utilities|Struct|BreakMagicElementMaterials MagicElementMaterials))
  (bind _ns_flare (Variables|Default|GetNS_Flare)
    (:then
      (Utilities|FlowControl|Sequence
        (:then_0
          (Class|NiagaraComponent|SetVariableMaterial _ns_flare "UserRibbonPrimaryMaterial" _magicelementmaterial))
        (:then_1
          (Class|NiagaraComponent|SetVariableMaterial _ns_flare "UserRibbonSecondaryMaterial" _magicelementmaterialemissive))
        (:then_2
          (Niagara|SetNiagaraVariable(LinearColor) _ns_flare "UserRibbonPrimaryColour" _magicprimarycolour))
        (:then_3
          (Niagara|SetNiagaraVariable(LinearColor) _ns_flare "UserRibbonSecondaryColour" _magicsecondarycolour))))
    (:else)))

(fn ApplyMeshes
  (params (Mesh :type Static%20Mesh%20Object%20Reference))
  (bind _spellmesh (Variables|Default|GetSpellMesh)
    (:then
      (Components|StaticMesh|SetStaticMesh _spellmesh Mesh)
      (bind _ns_spellburst (Variables|Default|GetNS_SpellBurst)
        (:then
          (Class|NiagaraComponent|SetVariableStaticMesh _ns_spellburst "BurstStaticMesh" Mesh))
        (:else)))
    (:else)))

(fn SetProjectileSpeeds
  (bind _projectilemovement (Variables|Default|GetProjectileMovement))
  (bind _output_get (Variables|/Script/Engine.ProjectileMovementComponent|SetMaxSpeed _projectilemovement (Variables|/Script/Sigil.DA_SpellInfo|GetSpeed (Variables|Default|GetSpellDataAsset))))
  (bind _output_get_2 (Variables|/Script/Engine.ProjectileMovementComponent|SetInitialSpeed _projectilemovement _output_get))
  (Variables|/Script/Engine.ProjectileMovementComponent|SetHomingAccelerationMagnitude _projectilemovement (* _output_get_2 1e+01)))

(fn ConfigureProjectileHoming
  (params (bIsHomingProjectile :type Boolean))
  (Variables|/Script/Engine.ProjectileMovementComponent|SetbIsHomingProjectile (Variables|Default|GetProjectileMovement) bIsHomingProjectile)
  (bind _targetcomponentref (Variables|Default|GetTargetComponentRef)
    (:then
      (Utilities|IsValid _targetcomponentref
        (:Is%20Valid
          (Variables|/Script/Engine.ProjectileMovementComponent|SetHomingTargetComponent (Variables|Default|GetProjectileMovement) _targetcomponentref))))
    (:else)))