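; BP_MagicTurret is a magic turret that repeatedly fires its loaded spell at the player.
; While active, Tick accumulates a delay against the casts-per-second rate, then spawns a BP_SpellProjectile at the Arrow's transform if a spell is loaded.
; Each projectile receives the spell and a target component obtained from the player pawn by interface message.
; The turret's mesh ignores the new projectile when moving.
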(event EventBeginPlay)

(event Collision|EventActorBeginOverlap
  (params (OtherActor :type Actor%20Object%20Reference)))

(event EventTick
  (params (DeltaSeconds :type Float%20%28single-precision%29))
  (if (Variables|Default|GetbIsActive)
    (bind _output_get (Variables|Default|SetCastDelay (+ (Variables|Default|GetCastDelay) DeltaSeconds)))
    (if (>= _output_get (/ 1.0 (Variables|Default|GetCastPerSecond)))
      (bind _loadedspell (Variables|Default|GetLoadedSpell)
        (:then
          (bind _returnvalue (Class|SigilTargetingInterface|GetTargetComponent(Message) (Game|Player|GetPlayerPawn 0)))
          (bind _returnvalue_2 (Game|SpawnActorfromClass "/Game/Sigil/Blueprints/Magic/Projectiles/BP_SpellProjectile.BP_SpellProjectile_C" (Transformation|GetWorldTransform (Variables|Default|GetArrow)) "Undefined" 0 _loadedspell _returnvalue 0))
          (Collision|IgnoreActorwhenMoving (Variables|Default|GetStaticMesh) _returnvalue_2 true)
          (Variables|Default|SetCastDelay 0.0))
        (:else)))))

(fn ConstructionScript)