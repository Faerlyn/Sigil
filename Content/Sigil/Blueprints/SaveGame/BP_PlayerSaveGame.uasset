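; Player save game that stores and restores the name, character transform, controller rotation, created spells and prepared spells.
; Created spells are saved as property data and rebuilt on load as new DA_SpellInfo objects.
; Prepared spells are split into slot-keyed maps: non-editable core spells keep data asset references, while player spells keep indices into the created spell list.
; LoadGame rebuilds created spells first, then resolves prepared slots against them.
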(fn SavePlayerSpells
  (params (InPlayerSpells :type Array%20of%20DA%20Spell%20Info%20Object%20References))
  ;[0.3 0 0.5 0.3] Get each element of PlayerSpells and save their spell properties to SavedPlayerSpells
  (Utilities|Array|Clear (Variables|SaveGame|Spells|PlayerSpells|GetSavedPlayerSpells))
  (for _array_element InPlayerSpells
    (bind _returnvalue (Class|DASpellInfo|GetSpellProperties _array_element))
    (Utilities|Array|Add (Variables|SaveGame|Spells|PlayerSpells|GetSavedPlayerSpells) _returnvalue)))

(fn LoadPlayerSpells
  ;[0.3 0 0.5 0.3] For each element of SavedPlayerSpells, create a DA_SpellInfo object and set its properties to that of the element. Store a reference to this object in OutPlayerSpells
  (Utilities|Array|Clear (Variables|SaveGame|Spells|PlayerSpells|GetOutPlayerSpells))
  (for _array_element (Variables|SaveGame|Spells|PlayerSpells|GetSavedPlayerSpells)
    (bind _returnvalue (Game|ConstructObjectfromClass "/Script/Sigil.DA_SpellInfo"))
    (Class|DASpellInfo|SetSpellProperties _returnvalue _array_element)
    (Utilities|Array|Add (Variables|SaveGame|Spells|PlayerSpells|GetOutPlayerSpells) _returnvalue))
  (return (Variables|SaveGame|Spells|PlayerSpells|GetOutPlayerSpells)))

(fn SavePreparedSpells
  (params (InPlayerSpells :type Array%20of%20DA%20Spell%20Info%20Object%20References) (InPreparedSpells :type Array%20of%20DA%20Spell%20Info%20Object%20References))
  ;[0.3 0 0.5 0.3] Clear PreparedCoreSpells and PreparedPlayerSpells
  (Utilities|Map|Clear (Variables|SaveGame|Spells|PreparedSpells|GetPreparedCoreSpells))
  (Utilities|Map|Clear (Variables|SaveGame|Spells|PreparedSpells|GetPreparedPlayerSpells))
  ;[0.3 0 0.5 0.3] If the element of PreparedSpells matches a player-created spell, save the indices PreparedSpells and PlayerSpells inside PreparedPlayerSpells.
  ; Now check if the element of PreparedSpells is not editable (this means that the spell is a Data Asset). If true, save the index and DA_SpellInfo reference to PreparedCoreSpells.
  (for (_array_element _array_index) InPreparedSpells
    (for (_array_element_2 _array_index_2) InPlayerSpells
      (if (== _array_element_2 _array_element)
        (Utilities|Map|Add (Variables|SaveGame|Spells|PreparedSpells|GetPreparedPlayerSpells) _array_index _array_index_2)))
    (if (not (Variables|/Script/Sigil.DA_SpellInfo|GetbCanEdit _array_element))
      (Utilities|Map|Add (Variables|SaveGame|Spells|PreparedSpells|GetPreparedCoreSpells) _array_index _array_element)))
  (Variables|SaveGame|Spells|PreparedSpells|SetPreparedSpellsLength (Utilities|Array|Length InPreparedSpells)))

(fn LoadPreparedSpells
  ;[0.3 0 0.5 0.3] Clear OutPreparedSpells
  (Utilities|Array|Clear (Variables|SaveGame|Spells|PreparedSpells|GetOutPreparedSpells))
  ;[0.3 0 0.5 0.3] Load the saved spell for each element of PreparedSpells
  (for _index (range 0 (Variables|SaveGame|Spells|PreparedSpells|GetPreparedSpellsLength))
    (bind _success (LoadGame|Spells|PreparedSpells|TryLoadPreparedCoreSpells _index))
    (if (not _success)
      _
      (else
        _))
    (LoadGame|Spells|PreparedSpells|TryLoadPreparedPlayerSpells _index))
  (return (Variables|SaveGame|Spells|PreparedSpells|GetOutPreparedSpells)))

(fn SaveGame
  (params (SaveSlotName :type String) (UserIndex :type Integer) (PlayerName :type Name) (PlayerCharacterTransform :type Transform) (PlayerControllerRotation :type Rotator) (PlayerSpells :type Array%20of%20DA%20Spell%20Info%20Object%20References) (PreparedSpells :type Array%20of%20DA%20Spell%20Info%20Object%20References))
  (Utilities|FlowControl|Sequence
    (:then_0
      (Variables|SaveGame||SetSavedSaveSlotName SaveSlotName))
    (:then_1
      (Variables|SaveGame||SetSavedUserIndex UserIndex))
    (:then_2
      (Variables|SaveGame|PlayerInfo|SetSavedPlayerName PlayerName))
    (:then_3
      (Variables|SaveGame|PlayerInfo|SetSavedPlayerCharacterTransform PlayerCharacterTransform))
    (:then_4
      (Variables|SaveGame|PlayerInfo|SetSavedPlayerControllerRotation PlayerControllerRotation))
    (:then_5
      (SaveGame|Spells|PlayerSpells|SavePlayerSpells PlayerSpells))
    (:then_6
      (SaveGame|Spells|PreparedSpells|SavePreparedSpells PlayerSpells PreparedSpells))))

(fn LoadGame
  (bind _outplayerspells (LoadGame|Spells|PlayerSpells|LoadPlayerSpells))
  (bind _outpreparedspells (LoadGame|Spells|PreparedSpells|LoadPreparedSpells))
  (return (Variables|SaveGame|PlayerInfo|GetSavedPlayerName) (Variables|SaveGame|PlayerInfo|GetSavedPlayerCharacterTransform) (Variables|SaveGame|PlayerInfo|GetSavedPlayerControllerRotation) _outplayerspells _outpreparedspells))

(fn TryLoadPreparedCoreSpells
  (params (PreparedSpellsIndex :type Integer%20%28by%20ref%29))
  (bind _preparedcorespells (Variables|SaveGame|Spells|PreparedSpells|GetPreparedCoreSpells))
  (bind (_value _returnvalue) (Utilities|Map|Find _preparedcorespells PreparedSpellsIndex))
  ;[0.3 0 0.5 0.3] If PreparedCoreSpells has an element at the provided index, add the spell to OutPreparedSpells at the same index
  (if _returnvalue
    (Utilities|Array|SetArrayElem (Variables|SaveGame|Spells|PreparedSpells|GetOutPreparedSpells) PreparedSpellsIndex _value true)
    (return true)
    (else
      (return false))))

(fn TryLoadPreparedPlayerSpells
  (params (PreparedSpellsIndex :type Integer%20%28by%20ref%29))
  (bind _preparedplayerspells (Variables|SaveGame|Spells|PreparedSpells|GetPreparedPlayerSpells))
  (bind (_value _returnvalue) (Utilities|Map|Find _preparedplayerspells PreparedSpellsIndex))
  ;[0.3 0 0.5 0.3] If PreparedPlayerSpells has an element at the provided index, get the spell from OutPlayerSpells using the value of PreparedPlayerSpells as the index, add the spell to OutPreparedSpells at the provided index
  (if _returnvalue
    (Utilities|Array|SetArrayElem (Variables|SaveGame|Spells|PreparedSpells|GetOutPreparedSpells) PreparedSpellsIndex (Utilities|Array|Get(acopy) (Variables|SaveGame|Spells|PlayerSpells|GetOutPlayerSpells) _value) true)
    (return true)
    (else
      (return false))))